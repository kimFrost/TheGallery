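; BP_HDRI is a configurable HDRI skybox actor with a rotating cubemap and a skylight.
; The construction script applies a dynamic MI_HDRI instance to the Skybox, sets cubemap, brightness, tint, contrast and initial rotation, then recaptures the skylight.
; Tick eases CurrentRotation toward 360 with FInterpTo at a scaled-down speed, so rotation slows as it approaches rather than looping, and writes it to the material.
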(event EventTick
  (params (DeltaSeconds :type Float%20%28single-precision%29))
  ;[1 1 1] Rotation Speed
  (bind _output_get (Variables|Default|SetCurrentRotation (Math|Interpolation|FInterpTo (Variables|Default|GetCurrentRotation) 3.6e+02 DeltaSeconds (/ (Variables|HDRI|GetHDRI_RotationSpeed) 1e+03))))
  (Rendering|Material|SetScalarParameterValue (Variables|HDRI|GetHDRI_MInst) "CubemapRotation" _output_get :!class /Script/Engine.MaterialInstanceDynamic))

(fn ConstructionScript
  (bind _skylight1 (Variables|BP_DayLight|GetSkyLight1))
  (Utilities|FlowControl|Sequence
    (:then_0
      ;[1 1 1] Material Instance
      (Transformation|SetWorldRotation (Variables|Default|GetSkybox) "0.000000, 0, 0" false false)
      (bind _returnvalue (Rendering|Material|CreateDynamicMaterialInstance "/Game/HDRIS/Materials/MI_HDRI.MI_HDRI" :!class /Script/Engine.KismetMaterialLibrary))
      (bind _output_get (Variables|HDRI|SetHDRI_MInst _returnvalue))
      ;[1 1 1] HDRI Parameters
      (Rendering|Material|SetMaterial (Variables|Default|GetSkybox) 0 _output_get)
      ;;[1 1 1] HDRI Brightness
      (Rendering|Material|SetScalarParameterValue (Variables|HDRI|GetHDRI_MInst) "HDRI_Brightness" (Variables|HDRI|GetHDRI_Brightness) :!class /Script/Engine.MaterialInstanceDynamic)
      (Rendering|Material|SetVectorParameterValue (Variables|HDRI|GetHDRI_MInst) "HDRI_Tint" (Variables|HDRI|GetHDRI_Tint) :!class /Script/Engine.MaterialInstanceDynamic)
      (Rendering|Material|SetTextureParameterValue (Variables|HDRI|GetHDRI_MInst) "HDRI_Cubemap" (Variables|HDRI|GetHDRI_Cubemap))
      ;;[1 1 1] Rotation
      (Rendering|Material|SetScalarParameterValue (Variables|HDRI|GetHDRI_MInst) "CubemapRotation" (Variables|HDRI|GetCubemapRotation) :!class /Script/Engine.MaterialInstanceDynamic)
      (Rendering|Material|SetScalarParameterValue (Variables|HDRI|GetHDRI_MInst) "HDRI_Contrast" (Variables|HDRI|GetHDRI_Contrast) :!class /Script/Engine.MaterialInstanceDynamic))
    (:then_1
      ;[1 1 1] Recapture Skylight
      (Class|SkyLightComponent|RecaptureSky _skylight1)
      (if (not true)
        (Components|DestroyComponent _skylight1)))))